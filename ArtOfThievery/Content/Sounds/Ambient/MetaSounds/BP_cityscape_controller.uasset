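; Controller Blueprint for city ambience that plays the ME_cityscape MetaSound and periodically sets off a car alarm within it.
; BeginPlay spawns the sound in 2D, keeps a reference to it and starts an initial cooldown.
; Tick counts the cooldown down, then fires the "Car alarm" trigger parameter and resets to a longer delay.
; The random roll gating the trigger spans its whole threshold, so it almost always passes.
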(event EventBeginPlay
  ;[1 1 1] Spawn the meta sound and create and initial car alarm cooldown
  (Variables|Default|SetCar%20alarm%20cooldown 2e+01)
  (bind _returnvalue (Audio|SpawnSound2D "/Game/Sounds/Ambient/MetaSounds/ME_cityscape.ME_cityscape" 1.0 1.0 0.0 0))
  (Variables|Default|Setmeta%20sound%20object _returnvalue))

(event Collision|EventActorBeginOverlap
  (params (OtherActor :type Actor%20Object%20Reference)))

(event EventTick
  (params (DeltaSeconds :type Float%20%28single-precision%29))
  ;[1 1 1] Check if the car alarm should be played
  (Variables|Default|SetCar%20alarm%20cooldown (- (Variables|Default|GetCar%20alarm%20cooldown) DeltaSeconds))
  (if (> 0.0 (Variables|Default|GetCar%20alarm%20cooldown))
    (if (> 1e+03 (Math|Random|RandomFloatinRange 0.0 1e+03))
      (Class|AudioParameterControllerInterface|SetTriggerParameter (Variables|Default|Getmeta%20sound%20object) "Car alarm")
      (Variables|Default|SetCar%20alarm%20cooldown 9e+01))))

(fn ConstructionScript)