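; Keypad code-lock minigame: the player, once in range, toggles into the keypad's view with the escape binding and clicks digits to unlock a Target.
; Mouse traces identify digits by each button's material and append them to a string, which is checked at the correct code's length.
; Results drive the status light and keypad sound triggers, and success calls Interact on Target.
; The pressed-button material flash is unconnected.
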(event Custom|LeftClick
  (bind _playercontroller (Variables|Default|GetPlayerController))
  (bind (_worldlocation _worlddirection) (Game|Player|ConvertMouseLocationToWorldSpace _playercontroller))
  (if (Variables|Default|Getactive)
    (bind _outhit (Collision|LineTraceByChannel _worldlocation (+ _worlddirection (* _worlddirection 1e+05)) "TraceTypeQuery2" false 0 "None" false))
    (Variables|Default|SetLatest%20hit%20location (.ImpactPoint (Collision|BreakHitResult _outhit)))
    (bind (_number_string _number_integer) (CallFunction|MaterialSwitch (Rendering|Material|GetMaterial (.HitComponent (Collision|BreakHitResult _outhit)) 0)))
    (if (!= _number_integer -1)
      (bind _output_get (Variables|Default|SetCode%20Input (Utilities|String|Append (Variables|Default|GetCode%20Input) _number_string)))
      (Development|PrintText (Utilities|Text|ToText(String) _output_get))
      (Utilities|FlowControl|Sequence
        (:then_0
          (Class|AudioParameterControllerInterface|SetTriggerParameter (Variables|Default|GetNewVar) "keyHit")
          (if (>= (Utilities|String|Len (Variables|Default|GetCode%20Input)) (Utilities|String|Len (Variables|Default|GetCorrect%20Code)))
            (if (Utilities|Enum|Equal(Enum) (Variables|Default|GetCode%20Input) (Variables|Default|GetCorrect%20Code))
              (Development|PrintText "Unlocked!")
              (Class|AudioParameterControllerInterface|SetTriggerParameter (Variables|Default|GetNewVar) "Granted")
              (Rendering|Material|SetMaterial (Variables|Default|Getstatus%20light) 0 "/Game/GameplayObjects/materials/ButtonPad/M_Code_corret.M_Code_corret")
              (Default|Interact (Variables|Default|GetTarget))
              (Variables|Default|SetCode%20Input "")
              (else
                (Development|PrintText "Wrong")
                (Variables|Default|SetCode%20Input "")
                (Rendering|Material|SetMaterial (Variables|Default|Getstatus%20light) 0 "/Game/GameplayObjects/materials/ButtonPad/M_Code_wrng.M_Code_wrng")
                (Class|AudioParameterControllerInterface|SetTriggerParameter (Variables|Default|GetNewVar) "Denied")
                (Utilities|FlowControl|Delay 3.0)
                (Rendering|Material|SetMaterial (Variables|Default|Getstatus%20light) 0 "/Game/GameplayObjects/materials/ButtonPad/M_Code_none.M_Code_none")))))))))

(event Custom|exit
  (if (Variables|Default|GetPlayerIsInRange)
    (if (Variables|Default|Getactive)
      (Game|Player|SetViewTargetwithBlend (Variables|Default|GetPlayerController) (Variables|Default|GetPlayer) 0.0 "VTBlend_Linear" 0.0 false)
      (Variables|/Script/Engine.PlayerController|SetbShowMouseCursor (Variables|Default|GetPlayerController) false)
      (Variables|Default|Setactive false)
      (Variables|/Game/ThirdPerson/Blueprints/BP_ThirdPersonCharacter.BP_ThirdPersonCharacter_C|SetIsActive (Variables|Default|GetPlayer) true)
      (else
        (Variables|/Game/ThirdPerson/Blueprints/BP_ThirdPersonCharacter.BP_ThirdPersonCharacter_C|SetIsActive (Variables|Default|GetPlayer) false)
        (Variables|Default|Setactive true)
        (bind _output_get (Variables|Default|SetPlayerController (Game|GetPlayerController 0)))
        (Game|Player|SetViewTargetwithBlend _output_get self 0.0 "VTBlend_Linear" 0.0 false)
        (Variables|/Script/Engine.PlayerController|SetbShowMouseCursor (Variables|Default|GetPlayerController) true)))))

(event EventBeginPlay
  (bind _button_5 (Variables|Default|Getbutton%205))
  (Rendering|Material|SetMaterial (Variables|Default|Getstatus%20light) 0 "/Game/GameplayObjects/materials/ButtonPad/M_Code_none.M_Code_none")
  (bind _returnvalue (Actor|GetActorOfClass "/Game/ThirdPerson/Blueprints/BP_ThirdPersonCharacter.BP_ThirdPersonCharacter_C"))
  (bind _output_get (Variables|Default|SetPlayer _returnvalue))
  (EventDispatchers|BindEventtoMouseclick _output_get (delegate Custom|LeftClick))
  (Variables|Default|Setactive false)
  (EventDispatchers|BindEventtoEscapePress (Variables|Default|GetPlayer) (delegate Custom|exit))
  (Variables|Default|SetPlayerIsInRange false)
  (Variables|/Script/Engine.SceneComponent|SetbAbsoluteLocation _button_5 true)
  (bind _returnvalue_2 (Audio|SpawnSoundatLocation "/Game/GameplayObjects/sounds/ME_keypad.ME_keypad" (Variables|/Script/Engine.SceneComponent|GetRelativeLocation _button_5) "0, 0, 0" 1.0 1.0 0.0 0 0))
  (Variables|Default|SetNewVar _returnvalue_2))

(event Collision|EventActorBeginOverlap
  (params (OtherActor :type Actor%20Object%20Reference))
  (if (== OtherActor (Variables|Default|GetPlayer))
    (Variables|Default|SetPlayerIsInRange true)))

(event EventTick
  (params (DeltaSeconds :type Float%20%28single-precision%29)))

(fn ConstructionScript)

(fn MaterialSwitch
  (params (Input%20Material :type Material%20Interface%20Object%20Reference))
  (LocalVariables|SetMaterial Input%20Material)
  (LocalVariables|SetOutput%20string "")
  (LocalVariables|SetOutput%20integer -1)
  (if (== Input%20Material "/Game/GameplayObjects/materials/ButtonPad/M_0.M_0")
    (LocalVariables|SetOutput%20string "0")
    (LocalVariables|SetOutput%20integer 0)
    (elif (== Input%20Material "/Game/GameplayObjects/materials/ButtonPad/M_1.M_1")
      (LocalVariables|SetOutput%20string "1")
      (LocalVariables|SetOutput%20integer 1)
      (elif (== (LocalVariables|GetMaterial) "/Game/GameplayObjects/materials/ButtonPad/M_2.M_2")
        (LocalVariables|SetOutput%20string "2")
        (LocalVariables|SetOutput%20integer 2)
        (elif (== (LocalVariables|GetMaterial) "/Game/GameplayObjects/materials/ButtonPad/M_3.M_3")
          (LocalVariables|SetOutput%20string "3")
          (LocalVariables|SetOutput%20integer 3)
          (elif (== (LocalVariables|GetMaterial) "/Game/GameplayObjects/materials/ButtonPad/M_4.M_4")
            (LocalVariables|SetOutput%20string "4")
            (LocalVariables|SetOutput%20integer 4)
            (elif (== (LocalVariables|GetMaterial) "/Game/GameplayObjects/materials/ButtonPad/M_5.M_5")
              (LocalVariables|SetOutput%20string "5")
              (LocalVariables|SetOutput%20integer 5)
              (elif (== (LocalVariables|GetMaterial) "/Game/GameplayObjects/materials/ButtonPad/M_6.M_6")
                (LocalVariables|SetOutput%20string "6")
                (LocalVariables|SetOutput%20integer 6)
                (elif (== (LocalVariables|GetMaterial) "/Game/GameplayObjects/materials/ButtonPad/M_7.M_7")
                  (LocalVariables|SetOutput%20string "7")
                  (LocalVariables|SetOutput%20integer 7)
                  (elif (== (LocalVariables|GetMaterial) "/Game/GameplayObjects/materials/ButtonPad/M_8.M_8")
                    (LocalVariables|SetOutput%20string "8")
                    (LocalVariables|SetOutput%20integer 8)
                    (elif (== (LocalVariables|GetMaterial) "/Game/GameplayObjects/materials/ButtonPad/M_9.M_9")
                      (LocalVariables|SetOutput%20string "9")
                      (LocalVariables|SetOutput%20integer 9)))))))))))
  (return (LocalVariables|GetOutput%20string) (LocalVariables|GetOutput%20integer)))

(fn GetPressedMaterial
  (params (Material :type Material%20Interface%20Object%20Reference))
  (bind _number_integer (CallFunction|MaterialSwitch Material))
  (switch int _number_integer
    (:0
      (return "/Game/GameplayObjects/materials/ButtonPad/M_0_grey.M_0_grey" "/Game/GameplayObjects/materials/ButtonPad/M_0.M_0"))
    (:1
      (return "/Game/GameplayObjects/materials/ButtonPad/M_1_grey.M_1_grey" "/Game/GameplayObjects/materials/ButtonPad/M_1.M_1"))
    (:2
      (return "/Game/GameplayObjects/materials/ButtonPad/M_2_grey.M_2_grey" "/Game/GameplayObjects/materials/ButtonPad/M_2.M_2"))
    (:3
      (return "/Game/GameplayObjects/materials/ButtonPad/M_3_grey.M_3_grey" "/Game/GameplayObjects/materials/ButtonPad/M_3.M_3"))
    (:4
      (return "/Game/GameplayObjects/materials/ButtonPad/M_4_grey.M_4_grey" "/Game/GameplayObjects/materials/ButtonPad/M_4.M_4"))
    (:5
      (return "/Game/GameplayObjects/materials/ButtonPad/M_5_grey.M_5_grey" "/Game/GameplayObjects/materials/ButtonPad/M_5.M_5"))
    (:6
      (return "/Game/GameplayObjects/materials/ButtonPad/M_6_grey.M_6_grey" "/Game/GameplayObjects/materials/ButtonPad/M_6.M_6"))
    (:7
      (return "/Game/GameplayObjects/materials/ButtonPad/M_7_grey.M_7_grey" "/Game/GameplayObjects/materials/ButtonPad/M_7.M_7"))
    (:8
      (return "/Game/GameplayObjects/materials/ButtonPad/M_8_grey.M_8_grey" "/Game/GameplayObjects/materials/ButtonPad/M_8.M_8"))
    (:9
      (return "/Game/GameplayObjects/materials/ButtonPad/M_9_grey.M_9_grey" "/Game/GameplayObjects/materials/ButtonPad/M_9.M_9"))))