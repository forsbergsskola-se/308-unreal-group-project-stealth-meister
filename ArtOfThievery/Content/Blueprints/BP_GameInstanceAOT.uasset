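; Game instance Blueprint that saves and restores the player character's transform through a BP_GameSaves object in a named save slot.
; GameSave creates the save object if none is cached, records player 0's transform and writes it to the slot.
; GameLoad reads the slot, or creates a fresh object when none exists, and in both cases applies its stored transform, so a new save moves the player to the default value.
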(event Custom|GameSave
  ;[0 1 1] Save Game
  (Utilities|IsValid (Variables|Default|GetSaveGame)
    (:Is%20Valid
      _)
    (:Is%20Not%20Valid
      (bind _returnvalue (SaveGame|CreateSaveGameObject "/Game/SavedGames/BP_GameSaves.BP_GameSaves_C"))
      (Variables|Default|SetSaveGame _returnvalue)))
  (Variables|/Game/SavedGames/BP_GameSaves.BP_GameSaves_C|SetLocation (Variables|Default|GetSaveGame) (Transformation|GetActorTransform (Game|GetPlayerCharacter 0)))
  (SaveGame|SaveGametoSlot (Variables|Default|GetSaveGame) (Variables|Default|GetSaveSlotName)))

(event Custom|GameLoad
  ;[0 1 1] Load Game
  (bind _returnvalue (SaveGame|DoesSaveGameExist (Variables|Default|GetSaveSlotName)))
  (if _returnvalue
    (bind _returnvalue_2 (SaveGame|LoadGamefromSlot (Variables|Default|GetSaveSlotName)))
    (bind _asbp_game_saves (Utilities|Casting|CastToBP_GameSaves _returnvalue_2))
    (Variables|Default|SetSaveGame _asbp_game_saves)
    (else
      (bind _returnvalue_3 (SaveGame|CreateSaveGameObject "/Game/SavedGames/BP_GameSaves.BP_GameSaves_C"))
      (Variables|Default|SetSaveGame _returnvalue_3)))
  (Transformation|SetActorTransform (Game|GetPlayerCharacter 0) (Variables|/Game/SavedGames/BP_GameSaves.BP_GameSaves_C|GetLocation (Variables|Default|GetSaveGame))))