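; BP_ThrowableObject01 is a soda can actor that the player can pick up and throw through Interact and Throw events.
; Pick Up registers it as the third-person character's HeldItem, disables collision, attaches it to the mesh's left item socket and sets IsHolding from the attach result.
; ThrowItem restores collision and enables physics on the can, but its impulse is zero and it never clears the held state.
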(event EventBeginPlay)

(event Collision|EventActorBeginOverlap
  (params (OtherActor :type Actor%20Object%20Reference)))

(event EventTick
  (params (DeltaSeconds :type Float%20%28single-precision%29)))

(event EventInteract
  (CallFunction|PickUp))

(event EventThrow
  (CallFunction|ThrowItem))

(fn ConstructionScript)

(fn PickUp
  ;[0 1 0] Pick Up
  (bind _asbp_third_person_character (Utilities|Casting|CastToBP_ThirdPersonCharacter (Game|GetPlayerCharacter 0)))
  (bind _output_get (Variables|/Game/ThirdPerson/Blueprints/BP_ThirdPersonCharacter.BP_ThirdPersonCharacter_C|SetHeldItem _asbp_third_person_character self))
  (Collision|SetActorEnableCollision false)
  (bind _returnvalue (Transformation|AttachComponentToComponent _output_get (Variables|/Script/Engine.Character|GetMesh _asbp_third_person_character) "ItemSocket_l" "SnapToTarget" "KeepRelative" "KeepRelative" true))
  (Variables|/Game/ThirdPerson/Blueprints/BP_ThirdPersonCharacter.BP_ThirdPersonCharacter_C|SetIsHolding _asbp_third_person_character _returnvalue))

(fn ThrowItem
  ;[0 1 0] Throw Item
  (Collision|SetActorEnableCollision true)
  (Physics|SetSimulatePhysics (Variables|Default|GetSM_SodaCan) true)
  (Physics|AddImpulse (Variables|Default|GetSM_SodaCan) "0, 0, 0" "None" true)
  (Development|PrintString "Thrown" true true "(R=0.000000,G=1.000000,B=0.000000,A=1.000000)"))