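; BP_BasementExitPoint is an interactable exit that sends the player from the basement to MuseumLevel.
; On Interact it writes a hardcoded spawn transform to BP_GameInstanceAOT's SpawnLocation, then opens the level by name; a failed game instance cast stops the travel.
; A Box overlap shows the Widget component while the player character is inside and hides it on exit.
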(event OnComponentBeginOverlap(Box)
  (params (OverlappedComponent :type Primitive%20Component%20Object%20Reference) (OtherActor :type Actor%20Object%20Reference) (OtherComp :type Primitive%20Component%20Object%20Reference) (OtherBodyIndex :type Integer) (bFromSweep :type Boolean) (SweepResult :type Hit%20Result%20Structure%20%28by%20ref%29))
  (if (== OtherActor (Game|GetPlayerCharacter 0))
    (Development|SetHiddeninGame (Variables|Default|GetWidget) false false)))

(event OnComponentEndOverlap(Box)
  (params (OverlappedComponent :type Primitive%20Component%20Object%20Reference) (OtherActor :type Actor%20Object%20Reference) (OtherComp :type Primitive%20Component%20Object%20Reference) (OtherBodyIndex :type Integer))
  (if (== (Game|GetPlayerCharacter 0) OtherActor)
    (Development|SetHiddeninGame (Variables|Default|GetWidget) true false)))

(event EventInteract
  (params (Interacting%20Actor :type Actor%20Object%20Reference))
  (bind _asbp_game_instance_aot (Utilities|Casting|CastToBP_GameInstanceAOT (Game|GetGameInstance)))
  (Variables|/Game/Blueprints/BP_GameInstanceAOT.BP_GameInstanceAOT_C|SetSpawnLocation _asbp_game_instance_aot (Math|Transform|MakeTransform "3960.000000,1740.000000,90.000000" "0, 0, 0" "1.000000,1.000000,1.000000"))
  (Game|OpenLevel(byName) "MuseumLevel"))

(fn ConstructionScript)