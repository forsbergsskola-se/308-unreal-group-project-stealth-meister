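; Male guard AI for a stealth game, driven by event-graph AIMoveTo calls that loop random-point patrols.
; Player light/dark events set IsLit, gating PawnSensing sightings that start a faster chase; a retriggerable delay resumes patrol once sightings stop.
; AIPerception stimuli from the player send the guard to investigate their location before patrolling again.
; Player overlap with the guard's capsule shows the Mission Failed screen and switches to UI-only input.
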(event OnSeePawn(PawnSensing)
  (params (Pawn :type Pawn%20Object%20Reference))
  ;[0 1 1] Has seen Player
  (if (Variables|Default|GetIsLit)
    (Development|PrintString "Stop ! I see you !" true true "(R=0.000000,G=0.000000,B=0.000000,A=1.000000)")
    (Utilities|Casting|CastToBP_ThirdPersonCharacter Pawn)
    (Utilities|FlowControl|Sequence
      (:then_0
        (Variables|Default|SetSeenPlayer? true)
        (CallFunction|FollowPlayer))
      (:then_1
        (Utilities|FlowControl|RetriggerableDelay 0.6)
        (Variables|Default|SetSeenPlayer? false)
        (CallFunction|Patrolling)))
    (else
      (Development|PrintString "You are Invisible !" true true "(R=0.000000,G=1.000000,B=0.000000,A=1.000000)"))))

(event OnComponentBeginOverlap(CapsuleComponent)
  (params (OverlappedComponent :type Primitive%20Component%20Object%20Reference) (OtherActor :type Actor%20Object%20Reference) (OtherComp :type Primitive%20Component%20Object%20Reference) (OtherBodyIndex :type Integer) (bFromSweep :type Boolean) (SweepResult :type Hit%20Result%20Structure%20%28by%20ref%29))
  (bind _returnvalue (Game|GetPlayerController 0))
  (Utilities|Casting|CastToBP_ThirdPersonCharacter OtherActor)
  (bind _returnvalue_2 (UserInterface|CreateWidget "/Game/UI/LevelFinished/BPW_LevelFinished.BPW_LevelFinished_C"))
  (UserInterface|Viewport|AddtoViewport _returnvalue_2 0)
  (Rendering|Components|TextRender|SetText (Variables|/Game/UI/LevelFinished/BPW_LevelFinished.BPW_LevelFinished_C|GetMissionStatusText _returnvalue_2) "Mission Failed")
  (Rendering|Components|TextRender|SetText (Variables|/Game/UI/LevelFinished/BPW_LevelFinished.BPW_LevelFinished_C|GetMoneyAmountText _returnvalue_2) "0")
  (Rendering|Components|TextRender|SetText (Variables|/Game/UI/LevelFinished/BPW_LevelFinished.BPW_LevelFinished_C|GetReputationAmountText _returnvalue_2) "0")
  (Input|SetInputModeUIOnly _returnvalue 0 "DoNotLock" false)
  (Variables|/Script/Engine.PlayerController|SetbShowMouseCursor _returnvalue true))

(event OnTargetPerceptionUpdated(AIPerception)
  (params (Actor :type Actor%20Object%20Reference) (Stimulus :type AI%20Stimulus%20Structure))
  (bind (_age _expirationage _strength _stimuluslocation _receiverlocation _tag _bsuccessfullysensed) (Utilities|Struct|BreakAIStimulus Stimulus))
  ;[0 1 1] AI Investigate Noise
  (if (Variables|Default|GetIsLit)
    (Development|PrintString "Stop ! I see you !" true true "(R=1.000000,G=1.000000,B=1.000000,A=1.000000)")
    (else
      (Development|PrintString "You are silent !" true true "(R=0.000000,G=1.000000,B=0.000000,A=1.000000)")))
  (Utilities|Casting|CastToBP_ThirdPersonCharacter Actor)
  (if _bsuccessfullysensed
    (Development|PrintString "I hear Something !?" true true "(R=1.000000,G=1.000000,B=0.000000,A=1.000000)")
    (Variables|Default|SetInvestigating? true)
    (AI|AIMoveTo self _stimuluslocation 0 5.0 false
      (:OnSuccess
        (Utilities|FlowControl|Delay 3.0)
        (Development|PrintString "Must have been nothing." true true "(R=0.000000,G=1.000000,B=0.000000,A=1.000000)")
        (Variables|Default|SetInvestigating? false))
      (:OnFail
        _))
    (CallFunction|Patrolling)))

(event Custom|Follow%20Player
  ;[0 1 1] Chase Player
  (if (Variables|Default|GetSeenPlayer?)
    (Variables|/Script/Engine.CharacterMovementComponent|SetMaxWalkSpeed (Variables|Character|GetCharacterMovement) (Variables|Default|GetChasePlayerSpeed))
    (AI|AIMoveTo self "0, 0, 0" (Game|GetPlayerCharacter 0) 5.0 false
      (:OnSuccess
        (Development|PrintString "You'rer Nicked !" true true "(R=1.000000,G=0.000000,B=0.000000,A=1.000000)"))
      (:OnFail
        (CallFunction|CheckifLoseSightOfPlayer)))))

(event Custom|Patrolling
  ;[0 1 1] Patrtol
  (Variables|/Script/Engine.CharacterMovementComponent|SetMaxWalkSpeed (Variables|Character|GetCharacterMovement) (Variables|Default|GetNormalWalkSpeed))
  (AI|AIMoveTo self (.RandomLocation (AI|Navigation|GetRandomReachablePointinRadius (Transformation|GetActorLocation) 3e+03 0 0)) 0 5.0 false
    (:OnSuccess
      (Utilities|FlowControl|Delay 3.0))
    (:OnFail
      _))
  (if (Variables|Default|GetInvestigating?)
    (CallFunction|Patrolling)
    (else
      (CallFunction|Patrolling))))

(event Custom|CheckIfLoseSightOfPlayer
  ;[0 1 1] Lose Sight of Player
  (if (Utilities|Array|ContainsItem (Class|AIPerceptionComponent|GetPerceivedActors (Variables|Default|GetAIPerception) "/Script/AIModule.AISense_Sight") (Game|GetPlayerCharacter 0))
    (CallFunction|FollowPlayer)
    (else
      (Variables|Default|SetSeenPlayer? false)
      (CallFunction|Patrolling))))

(event Custom|SetPlayerIsVisible
  ;[1 1 1] Bind Event
  (Variables|Default|SetIsLit true)
  (Development|PrintString "Is Visible" true true "(R=1.000000,G=1.000000,B=1.000000,A=1.000000)"))

(event Custom|SetPlayerIsHidden
  ;[1 1 1] Bind Event
  (Variables|Default|SetIsLit false)
  (Development|PrintString "Invisible" true true "(R=0.000000,G=0.000000,B=1.000000,A=1.000000)"))

(event EventBeginPlay
  ;[1 1 1] Bind Event
  (CallFunction|Patrolling)
  (bind _asbp_third_person_character (Utilities|Casting|CastToBP_ThirdPersonCharacter (Game|GetPlayerCharacter 0)))
  (EventDispatchers|BindEventtoIntheLight _asbp_third_person_character (delegate Custom|SetPlayerIsVisible))
  (EventDispatchers|BindEventtoIntheDark _asbp_third_person_character (delegate Custom|SetPlayerIsHidden)))

(fn ConstructionScript)