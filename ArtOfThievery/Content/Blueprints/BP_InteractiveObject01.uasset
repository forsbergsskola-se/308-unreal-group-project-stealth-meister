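; BP_InteractiveObject01 is an interactable item that the player character can pick up and hold.
; Overlapping its Collider toggles a prompt widget, shown only while the player character is in range.
; Interact calls PickUp, which registers the item as the ThirdPersonCharacter's HeldItem, disables its collision and attaches it to the mesh socket ItemSocket_l.
; The attachment result sets the character's IsHolding flag.
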(event OnComponentBeginOverlap(Collider)
  (params (OverlappedComponent :type Primitive%20Component%20Object%20Reference) (OtherActor :type Actor%20Object%20Reference) (OtherComp :type Primitive%20Component%20Object%20Reference) (OtherBodyIndex :type Integer) (bFromSweep :type Boolean) (SweepResult :type Hit%20Result%20Structure%20%28by%20ref%29))
  ;[0 1 1] Prompt Widget
  (if (== OtherActor (Game|GetPlayerCharacter 0))
    (Development|SetHiddeninGame (Variables|Default|GetPromptWidget) false false)))

(event OnComponentEndOverlap(Collider)
  (params (OverlappedComponent :type Primitive%20Component%20Object%20Reference) (OtherActor :type Actor%20Object%20Reference) (OtherComp :type Primitive%20Component%20Object%20Reference) (OtherBodyIndex :type Integer))
  ;[0 1 1] Prompt Widget
  (if (== (Game|GetPlayerCharacter 0) OtherActor)
    (Development|SetHiddeninGame (Variables|Default|GetPromptWidget) true false)))

(event EventInteract
  (params (Interacting%20Actor :type Actor%20Object%20Reference))
  (CallFunction|PickUp))

(fn ConstructionScript)

(fn PickUp
  ;[0 1 0] Pick Up
  (bind _asbp_third_person_character (Utilities|Casting|CastToBP_ThirdPersonCharacter (Game|GetPlayerCharacter 0)))
  (bind _output_get (Variables|/Game/ThirdPerson/Blueprints/BP_ThirdPersonCharacter.BP_ThirdPersonCharacter_C|SetHeldItem _asbp_third_person_character self))
  (Collision|SetActorEnableCollision false)
  (bind _returnvalue (Transformation|AttachComponentToComponent _output_get (Variables|/Script/Engine.Character|GetMesh _asbp_third_person_character) "ItemSocket_l" "SnapToTarget" "KeepRelative" "KeepRelative" true))
  (Variables|/Game/ThirdPerson/Blueprints/BP_ThirdPersonCharacter.BP_ThirdPersonCharacter_C|SetIsHolding _asbp_third_person_character _returnvalue))