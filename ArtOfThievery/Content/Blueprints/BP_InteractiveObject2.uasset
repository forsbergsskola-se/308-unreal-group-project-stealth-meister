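; Interactive world object that the third-person player can pick up and throw.
; Interact makes it the character's HeldItem, disables its collision and attaches it to the left-hand item socket on the character mesh, storing the attach result in IsHolding.
; Throw re-enables collision, turns on mesh physics and applies a fixed world-space velocity impulse, without clearing the character's held state.
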(event EventThrow
  (CallFunction|ThrowItem))

(event EventInteract
  (CallFunction|PickUp))

(fn ConstructionScript)

(fn PickUp
  ;[0 1 0] Pick Up
  (bind _asbp_third_person_character (Utilities|Casting|CastToBP_ThirdPersonCharacter (Game|GetPlayerCharacter 0)))
  (bind _output_get (Variables|/Game/ThirdPerson/Blueprints/BP_ThirdPersonCharacter.BP_ThirdPersonCharacter_C|SetHeldItem _asbp_third_person_character self))
  (Collision|SetActorEnableCollision false)
  (bind _returnvalue (Transformation|AttachComponentToComponent _output_get (Variables|/Script/Engine.Character|GetMesh _asbp_third_person_character) "ItemSocketLeft" "SnapToTarget" "KeepRelative" "KeepRelative" true))
  (bind _output_get_2 (Variables|/Game/ThirdPerson/Blueprints/BP_ThirdPersonCharacter.BP_ThirdPersonCharacter_C|SetIsHolding _asbp_third_person_character _returnvalue))
  (return _output_get_2))

(fn ThrowItem
  ;[0 1 0] Throw Item
  (Collision|SetActorEnableCollision true)
  (Physics|SetSimulatePhysics (Variables|Default|GetSM_Object) true)
  (Physics|AddImpulse (Variables|Default|GetSM_Object) "500.000000,500.000000,500.000000" "None" true)
  (Development|PrintString "Thrown"))