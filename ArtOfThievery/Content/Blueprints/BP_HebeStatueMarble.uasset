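; Throwable marble statue prop, apparently built from a soda can item, that the player picks up to make noise.
; An overlap collider toggles the interact prompt; Interact attaches it to the character's left-hand socket.
; Throw enables physics and launches it along the camera-to-item direction, with extra vertical strength.
; Its first non-player impact plays a can sound and reports a noise event instigated by the player.
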(event OnComponentBeginOverlap(InteractionCollider)
  (params (OverlappedComponent :type Primitive%20Component%20Object%20Reference) (OtherActor :type Actor%20Object%20Reference) (OtherComp :type Primitive%20Component%20Object%20Reference) (OtherBodyIndex :type Integer) (bFromSweep :type Boolean) (SweepResult :type Hit%20Result%20Structure%20%28by%20ref%29))
  ;[0 1 1] Prompt Widget
  (if (== OtherActor (Game|GetPlayerCharacter 0))
    (Development|SetHiddeninGame (Variables|Default|GetPromptWidget) false false)))

(event OnComponentEndOverlap(InteractionCollider)
  (params (OverlappedComponent :type Primitive%20Component%20Object%20Reference) (OtherActor :type Actor%20Object%20Reference) (OtherComp :type Primitive%20Component%20Object%20Reference) (OtherBodyIndex :type Integer))
  ;[0 1 1] Prompt Widget
  (if (== (Game|GetPlayerCharacter 0) OtherActor)
    (Development|SetHiddeninGame (Variables|Default|GetPromptWidget) true false)))

(event EventInteract
  (params (Interacting%20Actor :type Actor%20Object%20Reference))
  (CallFunction|PickUp))

(event EventThrow
  (CallFunction|ThrowItem))

(event Collision|EventHit
  (params (MyComp :type Primitive%20Component%20Object%20Reference) (Other :type Actor%20Object%20Reference) (OtherComp :type Primitive%20Component%20Object%20Reference) (bSelfMoved :type Boolean) (HitLocation :type Vector :default "0, 0, 0") (HitNormal :type Vector :default "0, 0, 0") (NormalImpulse :type Vector :default "0, 0, 0") (Hit :type Hit%20Result%20Structure%20%28by%20ref%29))
  (bind _returnvalue (Game|GetPlayerCharacter 0))
  ;[1 0 1] Noise on Impact
  (if (!= Other _returnvalue)
    (Utilities|FlowControl|DoOnce false
      (:Completed
        (Development|PrintString "Clank !" true true "(R=1.000000,G=0.000000,B=0.000000,A=1.000000)")
        (Audio|PlaySoundatLocation "/Game/Blueprints/SFX_SodaCanCue.SFX_SodaCanCue" HitLocation "0, 0, 0" 1.0 1.0 0.0 0 0 0 0)
        (Class|AISenseHearing|ReportNoiseEvent HitLocation 1e+02 _returnvalue 0.0 "None")))))

(fn ConstructionScript)

(fn PickUp
  ;[0 1 0] Pick Up
  (bind _asbp_third_person_character (Utilities|Casting|CastToBP_ThirdPersonCharacter (Game|GetPlayerCharacter 0)))
  (bind _output_get (Variables|/Game/ThirdPerson/Blueprints/BP_ThirdPersonCharacter.BP_ThirdPersonCharacter_C|SetHeldItem _asbp_third_person_character self))
  (Collision|SetActorEnableCollision false)
  (bind _returnvalue (Transformation|AttachComponentToComponent _output_get (Variables|/Script/Engine.Character|GetMesh _asbp_third_person_character) "ItemSocket_l" "SnapToTarget" "KeepRelative" "KeepRelative" true))
  (Variables|/Game/ThirdPerson/Blueprints/BP_ThirdPersonCharacter.BP_ThirdPersonCharacter_C|SetIsHolding _asbp_third_person_character _returnvalue))

(fn ThrowItem
  (bind _throwstrength (Variables|Default|GetThrowStrength))
  ;[0 1 0] Throw Item
  (bind _asbp_third_person_character (Utilities|Casting|CastToBP_ThirdPersonCharacter (Game|GetPlayerCharacter 0)))
  (Collision|SetActorEnableCollision true)
  (Physics|SetSimulatePhysics (Variables|Default|GetSM_SodaCan) true)
  (Physics|SetPhysicsLinearVelocity (Variables|Default|GetSM_SodaCan) (Math|Vector|MakeVector (* (.x (Math|Vector|GetUnitDirection(Vector) (Transformation|GetWorldLocation (Variables|/Script/ArtOfThievery.ArtOfThieveryCharacter|GetFollowCamera _asbp_third_person_character)) (Transformation|GetActorLocation self))) _throwstrength) (* (.y (Math|Vector|GetUnitDirection(Vector) (Transformation|GetWorldLocation (Variables|/Script/ArtOfThievery.ArtOfThieveryCharacter|GetFollowCamera _asbp_third_person_character)) (Transformation|GetActorLocation self))) _throwstrength) (* (.z (Math|Vector|GetUnitDirection(Vector) (Transformation|GetWorldLocation (Variables|/Script/ArtOfThievery.ArtOfThieveryCharacter|GetFollowCamera _asbp_third_person_character)) (Transformation|GetActorLocation self))) (* _throwstrength 1e+01))) false "None")
  (Development|PrintString "Thrown" true true "(R=0.000000,G=1.000000,B=0.000000,A=1.000000)"))