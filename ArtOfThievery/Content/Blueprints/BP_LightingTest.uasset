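; BP_LightingTest is a test Blueprint that tracks whether the player is illuminated or in darkness through actor overlap.
; Begin and end overlap events cast the other actor to BP_ThirdPersonCharacter, then set IsLit on or off and print a debug message.
; Both branches have a constant true condition, so their else paths never run.
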(event Collision|EventActorBeginOverlap
  (params (OtherActor :type Actor%20Object%20Reference))
  ;[1 1 1] Player is Illuminated
  (Utilities|Casting|CastToBP_ThirdPersonCharacter OtherActor)
  (if true
    (Variables|Default|SetIsLit true)
    (Development|PrintString "Lit Up" true true "(R=1.000000,G=1.000000,B=1.000000,A=1.000000)")
    (else
      (Variables|Default|SetIsLit false))))

(event Collision|EventActorEndOverlap
  (params (OtherActor :type Actor%20Object%20Reference))
  ;[0 0 0] Player in Darkness
  (Utilities|Casting|CastToBP_ThirdPersonCharacter OtherActor)
  (if true
    (Variables|Default|SetIsLit false)
    (Development|PrintString "Unlit")
    (else
      (Variables|Default|SetIsLit true))))

(fn ConstructionScript)