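; Female guard AI character that patrols random reachable points, chases the player on sight and investigates perceived stimuli.
; PawnSensing starts the chase, with a retriggerable delay returning it to patrol once sightings stop; reaching the player only prints an arrest message.
; AIPerception sends it to the stimulus location, pausing patrol through an Investigating flag.
; Also holds an inactive NPC interaction event and a move-align-and-play animation event that unpossesses the player controller.
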(event OnSeePawn(PawnSensing)
  (params (Pawn :type Pawn%20Object%20Reference))
  ;[0 1 1] Has seen Player
  (Development|PrintString "Stop ! I see you !" true true "(R=1.000000,G=1.000000,B=1.000000,A=1.000000)")
  (Utilities|Casting|CastToBP_ThirdPersonCharacter Pawn)
  (Utilities|FlowControl|Sequence
    (:then_0
      (Variables|Default|SetSeenPlayer? true)
      (CallFunction|FollowPlayer))
    (:then_1
      (Utilities|FlowControl|RetriggerableDelay 0.6)
      (Variables|Default|SetSeenPlayer? false)
      (CallFunction|Patrolling))))

(event OnTargetPerceptionUpdated(AIPerception)
  (params (Actor :type Actor%20Object%20Reference) (Stimulus :type AI%20Stimulus%20Structure))
  (bind (_age _expirationage _strength _stimuluslocation _receiverlocation _tag _bsuccessfullysensed) (Utilities|Struct|BreakAIStimulus Stimulus))
  ;[0 1 1] AI Detection
  (Utilities|Casting|CastToBP_ThirdPersonCharacter Actor)
  (if _bsuccessfullysensed
    (Development|PrintString "I hear something !?" true true "(R=1.000000,G=1.000000,B=0.000000,A=1.000000)")
    (Variables|Default|SetInvestigating? true)
    (AI|AIMoveTo self _stimuluslocation 0 5.0 false
      (:OnSuccess
        (Utilities|FlowControl|Delay 3.0)
        (Variables|Default|SetInvestigating? false))
      (:OnFail
        _))
    (CallFunction|Patrolling)))

(event Custom|FollowPlayer
  ;[0 1 1] Chase Player
  (if (Variables|Default|GetSeenPlayer?)
    (AI|AIMoveTo self "0, 0, 0" (Game|GetPlayerCharacter 0) 5.0 false
      (:OnSuccess
        (Development|PrintString "You're Under Arrest !" true true "(R=1.000000,G=0.000000,B=0.000000,A=1.000000)"))
      (:OnFail
        (CallFunction|Patrolling)))))

(event Custom|Patrolling
  ;[0 1 1] Patrtol
  (AI|AIMoveTo self (.RandomLocation (AI|Navigation|GetRandomReachablePointinRadius (Transformation|GetActorLocation) 0.0 0 0)) 0 5.0 false
    (:OnSuccess
      (Utilities|FlowControl|Delay 3.0))
    (:OnFail
      _))
  (if (not (Variables|Default|GetInvestigating?))
    (CallFunction|Patrolling)))

(event EventStartAnimation
  (params (Animation :type Skeletal%20Mesh%20Component%20Object%20Reference) (Location :type Vector :default "0, 0, 0"))
  (bind _returnvalue (Transformation|GetActorTransform))
  (bind _mesh (Variables|Character|GetMesh))
  ;[0 0 0] NPC Interaction - Not Active
  (Pawn|UnPossess (Game|GetPlayerController 0))
  (Pawn|SpawnDefaultController)
  (AI|AIMoveTo self Location 0 5.0 false
    (:OnSuccess
      (Components|MoveComponentTo (Variables|Character|GetMesh) (Math|Transform|InverseTransformLocation _returnvalue (Transformation|GetWorldLocation Animation)) (Math|Transform|InverseTransformRotation _returnvalue (Transformation|GetWorldRotation Animation)) false false 0.5 false)
      (Components|Animation|SetAnimationMode _mesh "AnimationBlueprint")
      (Components|Animation|PlayAnimation _mesh (.animtoplay (Variables|/Script/Engine.SkeletalMeshComponent|GetAnimationData Animation)) false))))

(event EventNPCInteract
  (params (InteractingNPC :type Character%20Object%20Reference))
  ;[0 0 0] NPC Interaction - Not Active
  (bind _array_element (Utilities|Array|ForEachLoopwithBreak (Collision|GetOverlappingActors "/Script/Engine.Actor" :!class /Script/Engine.Actor) :!label _label)
    (:LoopBody
      (if (Utilities|DoesObjectImplementInterface _array_element "/Game/Blueprints/IBP_NPCInteractor.IBP_NPCInteractor_C")
        (Class|IBPNPCInteractor|NPCInteract(Message) _array_element)
        (goto _label Break)))))

(fn ConstructionScript)